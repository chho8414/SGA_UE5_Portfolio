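; Test player character Blueprint that handles crafting and inventory UI, with partial hunger and weapon logic.
; Keys 1 and I toggle crafting and inventory widgets, 2 prints item quantities, and F toggles crafting near the first found BP_CraftingTable.
; DrainStarving increments hunger and updates the HUD, but its timer and HUD setup are disconnected.
; PlayerWeapon destroys Mesh and attaches a hard-coded BP_Bat, whatever valid weapon is passed.
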(event `Key|One`
  (params (Key :type "Key Structure"))
  ; 제작 UI
  (:`Pressed`
    (`/Engine/EditorBlueprintResources/StandardMacros.FlipFlop`
      (:`A`
        (bind _returnvalue (`|CreateWidget` "/Game/UI/WB_CraftingMenu.WB_CraftingMenu_C"))
        (bind _output_get (set `self.CraftingMenu` _returnvalue))
        (`UserWidget.AddToViewport` _output_get 0))
      (:`B`
        (`Widget.SetVisibility` (`self.CraftingMenu`) "Hidden")))))

(event `Key|Two`
  (params (Key :type "Key Structure"))
  ; 인벤토리 인덱스 출력 (테스트용)
  (:`Pressed`
    (for _array_element (`/Game/TopDown/Blueprints/BP_InventoryComponent.Item` (`self.BP_InventoryComponent`))
      (`KismetSystemLibrary.PrintString` (`KismetTextLibrary.Conv_TextToString` (`KismetTextLibrary.Conv_IntToText` (`.Quantity_11_002201B14E48EFD6085791B5B1B688E2` (break `/Game/Inventory/ST_ItemStruct` _array_element))))))))

(event `Key|I`
  (params (Key :type "Key Structure"))
  ; 인벤토리 UI
  (:`Pressed`
    (`/Engine/EditorBlueprintResources/StandardMacros.FlipFlop`
      (:`A`
        (bind _returnvalue (`|CreateWidget` "/Game/UI/BP_Inventory.BP_Inventory_C"))
        (bind _output_get (set `self.Inventory` _returnvalue))
        (`UserWidget.AddToViewport` _output_get 0))
      (:`B`
        (`Widget.SetVisibility` (`self.Inventory`) "Hidden")))))

(event `self.ReceiveBeginPlay`
  ; 배고픔 게이지
)

(event `Key|F`
  (params (Key :type "Key Structure"))
  ; 아이템스폰(플레이어 손 위치)
)

(event `Key|F`
  (params (Key :type "Key Structure"))
  ; 제작 테이블 UI 상호작용
  (:`Pressed`
    (bind _outactors (`GameplayStatics.GetAllActorsOfClass` "/Game/Crafting/BP_CraftingTable.BP_CraftingTable_C"))
    (bind _asbp_crafting_table (cast `/Game/Crafting/BP_CraftingTable` (`|GetArrayItem` _outactors)))
    (if (`/Game/Crafting/BP_CraftingTable.isNearTable` _asbp_crafting_table)
      (if (`self.CraftingUIOpen`)
        (`Widget.RemoveFromParent` (`self.CraftingUIRef`))
        (set `self.CraftingUIOpen` false)
        (else
          (bind _returnvalue (`|CreateWidget` "/Game/UI/WB_CraftingMenu.WB_CraftingMenu_C"))
          (bind _output_get (set `self.CraftingUIRef` _returnvalue))
          (`UserWidget.AddToViewport` _output_get 0)
          (set `self.CraftingUIOpen` true))))))

(fn `DrainStarving`
  (`/Engine/EditorBlueprintResources/StandardMacros.IncrementFloat` (`self.Starving`)
    (:`  `
      (`ProgressBar.SetPercent` (`/Game/UI/BP_HUD.Starving` (`self.HUDRef`)) (/ (`self.Starving`) (`self.StarvingMax`)))
      (return))))

(fn `PlayerWeapon`
  (params (NewWeapon :type "Actor Object Reference"))
  (`/Engine/EditorBlueprintResources/StandardMacros.IsValid` NewWeapon
    (:`Is Valid`
      (`ActorComponent.K2_DestroyComponent` (`self.Mesh`))
      (bind _returnvalue (`|SpawnActorFromClass` "/Game/Pandazole_Survival_Crafting_Pack/Weapons/BP_Bat.BP_Bat_C" (`SceneComponent.GetSocketTransform` (`self.Mesh`) "None" "RTS_World") "Undefined" "MultiplyWithRoot" null null))
      (bind _output_get (set `self.EquippedWeapon` _returnvalue))
      (`self.K2_AttachToComponent` _output_get (`self.ItemSocket`) "ItemSocket" "SnapToTarget" "SnapToTarget" "SnapToTarget" true)
      (set `self.CurrentWeapon` (`local.NewWeapon`)))))

(fn `UserConstructionScript`)