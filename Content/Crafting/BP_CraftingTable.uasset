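; BP_CraftingTable is a crafting table actor that shows a widget when the top-down player character comes near it.
; Its Sphere component's begin and end overlap events cast the other actor to BP_TopDownCharacter and set the IsNearTable flag.
; That flag then drives the Widget component's visibility, without propagating to child components.
; No crafting logic is present; the graph handles only proximity detection.
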(event OnComponentBeginOverlap(Sphere)
  (params (OverlappedComponent :type Primitive%20Component%20Object%20Reference) (OtherActor :type Actor%20Object%20Reference) (OtherComp :type Primitive%20Component%20Object%20Reference) (OtherBodyIndex :type Integer) (bFromSweep :type Boolean) (SweepResult :type Hit%20Result%20Structure%20%28by%20ref%29))
  (Utilities|Casting|CastToBP_TopDownCharacter OtherActor)
  (if (stale _bsuccess)
    (bind _output_get (Variables|Default|SetisNearTable true))
    (Rendering|SetVisibility (Variables|Default|GetWidget) _output_get false)))

(event OnComponentEndOverlap(Sphere)
  (params (OverlappedComponent :type Primitive%20Component%20Object%20Reference) (OtherActor :type Actor%20Object%20Reference) (OtherComp :type Primitive%20Component%20Object%20Reference) (OtherBodyIndex :type Integer))
  (Utilities|Casting|CastToBP_TopDownCharacter OtherActor)
  (if (stale _bsuccess)
    (bind _output_get (Variables|Default|SetisNearTable false))
    (Rendering|SetVisibility (Variables|Default|GetWidget) _output_get false)))

(fn ConstructionScript)